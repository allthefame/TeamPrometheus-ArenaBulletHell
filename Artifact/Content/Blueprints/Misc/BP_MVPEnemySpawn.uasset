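; Bare-bones enemy spawner actor that keeps adding BP_Enemy_Base enemies to the level while the hero is alive.
; A looping timer from BeginPlay calls SpawnEnemies, which picks a random point inside the Bounds box at its center height.
; The timer pauses on player death, caught both by a bound death event and by polling the hero's damage component on Tick.
; The respawn-on-enemy-death binding is disconnected.
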(event Custom|OnDeathEvent
  (CallFunction|SpawnEnemies "/Game/Blueprints/Characters/Enemies/BP_Enemy_Base.BP_Enemy_Base_C"))

(event Custom|SpawnEnemiesEvent
  (CallFunction|SpawnEnemies "/Game/Blueprints/Characters/Enemies/BP_Enemy_Base.BP_Enemy_Base_C"))

(event Custom|PlayerDeathEvent
  (Utilities|Time|PauseTimerbyHandle (Variables|Default|GetEnemySpawnTimer)))

(event EventBeginPlay
  (bind _asbp_hero_base (Utilities|Casting|CastToBP_Hero_Base (Game|GetPlayerCharacter 0)))
  (Variables|Default|SetHeroRef _asbp_hero_base)
  (bind _returnvalue (Utilities|Time|SetTimerbyEvent (delegate Custom|SpawnEnemiesEvent) 2.0 true))
  (Variables|Default|SetEnemySpawnTimer _returnvalue)
  (EventDispatchers|BindEventtoOnPlayerDeath (delegate Custom|PlayerDeathEvent)))

(event Collision|EventActorBeginOverlap
  (params (OtherActor :type Actor%20Object%20Reference)))

(event EventTick
  (params (DeltaSeconds :type Float%20%28single-precision%29))
  (if (Variables|/Game/Blueprints/Components/BPC_DamageSystem.BPC_DamageSystem_C|GetIsDead (Variables|/Game/Blueprints/Characters/BP_Character_Base.BP_Character_Base_C|GetBPC_DamageSystem (Variables|Default|GetHeroRef)))
    (CallFunction|PlayerDeathEvent)))

(fn ConstructionScript
  (bind _bounds (Variables|Default|GetBounds))
  (bind _boxextent (Variables|/Script/Engine.BoxComponent|GetBoxExtent _bounds))
  (Variables|Default|SetSpawnBounds (Math|Vector2D|MakeVector2D (.x _boxextent) (.y _boxextent))))

(fn CheckifWaveActive
  (return (Utilities|Array|IsNotEmpty (Variables|Default|GetAliveEnemies))))

(fn SpawnEnemies
  (params (EnemyType :type BP%20Enemy%20Base%20Class%20Reference))
  (bind _bounds (Variables|Default|GetBounds))
  (bind _returnvalue (Transformation|GetWorldLocation _bounds))
  (bind _returnvalue_2 (Components|Box|GetScaledBoxExtent _bounds))
  (bind _returnvalue_3 (Math|Random|RandomPointinBoundingBox _returnvalue _returnvalue_2))
  (LocalVariables|SetLocalEnemyType EnemyType)
  (Game|SpawnActorfromClass (LocalVariables|GetLocalEnemyType) (Math|Transform|MakeTransform (Math|Vector|MakeVector (.x _returnvalue_3) (.y _returnvalue_3) (.z (Transformation|GetWorldLocation _bounds))) "0, 0, 0" "1.000000,1.000000,1.000000") "Undefined" "MultiplyWithRoot" 0 0))