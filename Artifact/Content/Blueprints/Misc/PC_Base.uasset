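; PC_Base is a player controller that handles left and right rotation input for the hero character.
; On BeginPlay it casts the first player pawn to BP_Hero_Base and caches it.
; The IA_Rotate_Right and IA_Rotate_Left Enhanced Input actions set control rotation from the hero capsule's world rotation, nudging yaw one degree either way per trigger.
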(event Input|EnhancedActionEvents|EnhancedInputActionIA_Rotate_Right
  (params (ActionValue :type Boolean) (ElapsedSeconds :type Float%20%28double-precision%29) (TriggeredSeconds :type Float%20%28double-precision%29) (InputAction :type Input%20Action%20Object%20Reference :default "/Game/Blueprints/Inputs/IA_Rotate_Right.IA_Rotate_Right"))
  (bind _as_bp_hero_base (Variables|Default|GetAs%20BP%20Hero%20Base))
  (bind _capsulecomponent (Variables|/Script/Engine.Character|GetCapsuleComponent _as_bp_hero_base))
  (bind _returnvalue (Transformation|GetWorldRotation _capsulecomponent))
  (Pawn|SetControlRotation (Math|Rotator|MakeRotator (.roll _returnvalue) (.pitch _returnvalue) (+ (.yaw _returnvalue) 1.0))))

(event Input|EnhancedActionEvents|EnhancedInputActionIA_Rotate_Left
  (params (ActionValue :type Boolean) (ElapsedSeconds :type Float%20%28double-precision%29) (TriggeredSeconds :type Float%20%28double-precision%29) (InputAction :type Input%20Action%20Object%20Reference :default "/Game/Blueprints/Inputs/IA_Rotate_Left.IA_Rotate_Left"))
  (bind _as_bp_hero_base (Variables|Default|GetAs%20BP%20Hero%20Base))
  (bind _capsulecomponent (Variables|/Script/Engine.Character|GetCapsuleComponent _as_bp_hero_base))
  (bind _returnvalue (Transformation|GetWorldRotation _capsulecomponent))
  (Pawn|SetControlRotation (Math|Rotator|MakeRotator (.roll _returnvalue) (.pitch _returnvalue) (+ (.yaw _returnvalue) -1.0))))

(event EventBeginPlay
  (bind _asbp_hero_base (Utilities|Casting|CastToBP_Hero_Base (Game|Player|GetPlayerPawn 0)))
  (Variables|Default|SetAs%20BP%20Hero%20Base _asbp_hero_base))

(event EventTick
  (params (DeltaSeconds :type Float%20%28single-precision%29)))

(fn ConstructionScript)