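; BP_Enemy_Base is a base enemy Blueprint with contact damage, a simple projectile attack and death handling.
; Overlapping its DamageCollision deals damage to BP_Hero_Base actors through their BPCDamageSystem component.
; SimpleAttack spawns a BP_EnemyBaseProj at the capsule's location and rotation.
; Its own BPCDamageSystem signals death, which stops the AI brain logic and destroys the actor.
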(event OnComponentBeginOverlap(DamageCollision)
  (params (OverlappedComponent :type Primitive%20Component%20Object%20Reference) (OtherActor :type Actor%20Object%20Reference) (OtherComp :type Primitive%20Component%20Object%20Reference) (OtherBodyIndex :type Integer) (bFromSweep :type Boolean) (SweepResult :type Hit%20Result%20Structure%20%28by%20ref%29))
  (bind _asbp_hero_base (Utilities|Casting|CastToBP_Hero_Base OtherActor))
  (Default|TakeDamage (Variables|/Game/Blueprints/Characters/BP_Character_Base.BP_Character_Base_C|GetBPC_DamageSystem _asbp_hero_base) (Utilities|Struct|MakeS_DamageInfo 1.0 false false false)))

(event Custom|SimpleAttack
  (bind _capsulecomponent (Variables|Default|GetCapsuleComponent))
  (bind _returnvalue (Transformation|GetWorldTransform _capsulecomponent))
  (Game|SpawnActorfromClass "/Game/Blueprints/Weapons/Projectiles/BP_EnemyBaseProj.BP_EnemyBaseProj_C" (Math|Transform|MakeTransform (.location _returnvalue) (.rotation _returnvalue) "1.000000,1.000000,1.000000") "Undefined" "MultiplyWithRoot" 0 0))

(event Custom|OnDeathEvent
  (Development|PrintString "Enemy Dead")
  (AI|Logic|StopLogic (Variables|/Script/AIModule.AIController|GetBrainComponent (AI|GetAIController self)) "")
  (Actor|DestroyActor))

(event EventBeginPlay
  (|CallParentFunction)
  (EventDispatchers|AssignOnDeath (Variables|Default|GetBPC_DamageSystem) (delegate Custom|OnDeathEvent)))

(fn ConstructionScript
  (|CallParentFunction))

(fn GetReference
  (return self))