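; Base player hero Blueprint that handles movement input and carries a damage system component.
; On controller change it adds the default Enhanced Input mapping context, and IA_Move drives movement along the control rotation's forward and right vectors.
; Debug keys H and J print health and apply test damage through BPCDamageSystem.
; The attack input is an empty stub, and the sword spawn and swing-like rotation nodes are unconnected.
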(event Input|EnhancedActionEvents|EnhancedInputActionIA_Move
  (params (ActionValue :type Vector%202D%20Structure) (ElapsedSeconds :type Float%20%28double-precision%29) (TriggeredSeconds :type Float%20%28double-precision%29) (InputAction :type Input%20Action%20Object%20Reference :default "/Game/Blueprints/Inputs/IA_Move.IA_Move"))
  (bind _returnvalue (Pawn|GetControlRotation :!class /Script/Engine.Pawn))
  (bind _returnvalue_2 (Pawn|GetControlRotation :!class /Script/Engine.Pawn))
  (Pawn|Input|AddMovementInput (Math|Vector|GetRightVector (Math|Rotator|MakeRotator (.roll _returnvalue_2) (.pitch _returnvalue_2) (.yaw _returnvalue_2))) (.x ActionValue) false)
  (Pawn|Input|AddMovementInput (Math|Vector|GetForwardVector (Math|Rotator|MakeRotator (.roll _returnvalue) (.pitch _returnvalue) (.yaw _returnvalue))) (.y ActionValue) false))

(event Input|EnhancedActionEvents|EnhancedInputActionIA_AttackAction
  (params (ActionValue :type Boolean) (ElapsedSeconds :type Float%20%28double-precision%29) (TriggeredSeconds :type Float%20%28double-precision%29) (InputAction :type Input%20Action%20Object%20Reference :default "/Game/Blueprints/Inputs/IA_AttackAction.IA_AttackAction"))
  ;[0.15 0.15 0.15 0.5] Attacking
)

(event EventBeginPlay
  (|CallParentFunction) ; This node is disabled and will not be called.\nDrag off pins to build functionality.
)

(event EventControllerChanged
  (params (OldController :type Controller%20Object%20Reference) (NewController :type Controller%20Object%20Reference))
  (bind _asplayer_controller (Utilities|Casting|CastToPlayerController NewController))
  (Input|AddMappingContext (PlayerController|LocalPlayerSubsystems|GetEnhancedInputLocalPlayerSubsystem _asplayer_controller) "/Game/Blueprints/Inputs/IMC_Default.IMC_Default" 0 "(bIgnoreAllPressedKeysUntilRelease=True,bForceImmediately=False,bNotifyUserSettings=False)"))

(event EventTick
  (params (DeltaSeconds :type Float%20%28single-precision%29))
  (|CallParentFunction DeltaSeconds) ; This node is disabled and will not be called.\nDrag off pins to build functionality.
)

(event Collision|EventActorBeginOverlap
  (params (OtherActor :type Actor%20Object%20Reference))
  (|CallParentFunction OtherActor) ; This node is disabled and will not be called.\nDrag off pins to build functionality.
)

(event Input|KeyboardEvents|DebugKey9
  (params (Key :type Key%20Structure :default "None") (ActionValue :type Input%20Action%20Value%20Structure))
  ;[0.15 0.15 0.15 0.5] Spawn Sword DEBUG
)

(event Input|KeyboardEvents|DebugKeyH
  (params (Key :type Key%20Structure :default "None") (ActionValue :type Input%20Action%20Value%20Structure))
  (bind _bpc_damagesystem (Variables|Default|GetBPC_DamageSystem))
  ;[0.15 0.15 0.15 0.5] Damage System Proof DEBUG
  (:Pressed
    (Development|PrintString (Utilities|String|ToString(Text) (Utilities|Text|FormatText "Player Health: {CurHealth}/{MaxHealth}" (Variables|/Game/Blueprints/Components/BPC_DamageSystem.BPC_DamageSystem_C|GetCurHealth _bpc_damagesystem) (Variables|/Game/Blueprints/Components/BPC_DamageSystem.BPC_DamageSystem_C|GetMaxHealth _bpc_damagesystem))))))

(event Input|KeyboardEvents|DebugKeyJ
  (params (Key :type Key%20Structure :default "None") (ActionValue :type Input%20Action%20Value%20Structure))
  ;[0.15 0.15 0.15 0.5] Damage System Proof DEBUG
  (:Pressed
    (bind _wasdamaged (Default|TakeDamage (Variables|Default|GetBPC_DamageSystem) (Utilities|Struct|MakeS_DamageInfo 1.0 false false false)))
    (if _wasdamaged
      (Development|PrintString "Player was dealt 1 damage =-(")
      (else
        (Development|PrintString "Player is DEAD X-P")))))

(fn ConstructionScript
  (|CallParentFunction))