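; BPC_DamageSystem is an actor component that handles health, damage and death for its BP_Character_Base owner.
; TakeDamage uses a CanBeDamaged macro to branch on dead, invincible and blocking states, honoring per-hit override flags, and returns whether damage landed.
; Applied damage lowers health, fires either the death or health-update dispatcher, and prints a debug message.
; The component also binds its own health-update event on BeginPlay.
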(event Custom|UpdateHealthEvent
  (params (CurHealth :type Float%20%28double-precision%29) (MaxHealth :type Float%20%28double-precision%29))
  (Utilities|IsValid (Variables|Default|GetEntityRef)
    (:Is%20Valid
      (Variables|Default|SetCurHealth CurHealth)
      (Variables|Default|SetMaxHealth MaxHealth))))

(event EventBeginPlay
  (bind _asbp_character_base (Utilities|Casting|CastToBP_Character_Base (Components|GetOwner)))
  (Variables|Default|SetEntityRef _asbp_character_base)
  (EventDispatchers|BindEventtoUpdateHealth (delegate Custom|UpdateHealthEvent)))

(fn TakeDamage
  (params (DamageInfo :type S%20Damage%20Info%20Structure))
  (bind (_amount _damagetype_ _canbeblocked _shoulddamageinvincible) (Utilities|Struct|BreakS_DamageInfo DamageInfo))
  (LocalVariables|SetLocalDamageDealt _amount)
  (Utilities|CanbeDamaged _canbeblocked _shoulddamageinvincible
    (:Block%20Damage
      (return false))
    (:Do%20Damage
      (bind _output_get (Variables|Default|SetCurHealth (- (Variables|Default|GetCurHealth) (LocalVariables|GetLocalDamageDealt))))
      (if (<= _output_get 0.0)
        (Variables|Default|SetIsDead true)
        (Default|CallOnDeath)
        (else
          (Default|CallUpdateHealth (Variables|Default|GetCurHealth) (Variables|Default|GetMaxHealth))))
      (Development|PrintString (Utilities|String|ToString(Text) (Utilities|Text|FormatText "Player was dealt {Damage} damage 
New Health: {CurHealth}/{MaxHealth}" (LocalVariables|GetLocalDamageDealt) (Variables|Default|GetCurHealth) (Variables|Default|GetMaxHealth))))
      (return true))
    (:No%20Damage
      (return false))))