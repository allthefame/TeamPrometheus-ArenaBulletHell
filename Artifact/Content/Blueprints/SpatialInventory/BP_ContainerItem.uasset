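; BP_ContainerItem describes a container item for the spatial inventory, exposing its name, thumbnail, grid size, container rows, actions and actor to spawn.
; Rotate toggles a Rotated flag, which GetThumbnail and GetDimensions read to return the rotated thumbnail and swapped X and Y dimensions.
; The remaining functions are plain getters over stored variables.
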(fn GetRows
  (return (Variables|Default|GetContainerRows)))

(fn GetName
  (return (Variables|Default|GetName)))

(fn GetThumbnail
  (if (Variables|Default|GetRotated)
    (return (Variables|Default|GetThumbnailRotated))
    (else
      (return (Variables|Default|GetThumbnail)))))

(fn GetDimensions
  (bind _dimension (Variables|Default|GetDimension))
  (if (Variables|Default|GetRotated)
    (return (Utilities|Struct|MakeIntPoint (.y _dimension) (.x _dimension)))
    (else
      (return (Variables|Default|GetDimension)))))

(fn Rotate
  (Variables|Default|SetRotated (not (Variables|Default|GetRotated)))
  (return))

(fn GetActortoSpawn
  (return (Variables|Default|GetActorToSpawn)))

(fn GetActions
  (return (Variables|Default|GetActions)))