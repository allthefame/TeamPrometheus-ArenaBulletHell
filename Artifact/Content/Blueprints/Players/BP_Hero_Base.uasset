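; Base hero character Blueprint that handles player movement and a simple melee swing through Enhanced Input.
; On controller change it adds the default mapping context, and IA_Move drives movement relative to control rotation.
; Each attack press alternates through a FlipFlop, instantly yawing MeleePivot one way or back, with no animation.
; A debug key spawns BP_Sword_Base at an offset from WeaponSpawn and attaches it to that component.
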(event Input|EnhancedActionEvents|EnhancedInputActionIA_Move
  (params (ActionValue :type Vector%202D%20Structure) (ElapsedSeconds :type Float%20%28double-precision%29) (TriggeredSeconds :type Float%20%28double-precision%29) (InputAction :type Input%20Action%20Object%20Reference :default "/Game/Blueprints/Inputs/IA_Move.IA_Move"))
  (bind _returnvalue (Pawn|GetControlRotation :!class /Script/Engine.Pawn))
  (bind _returnvalue_2 (Pawn|GetControlRotation :!class /Script/Engine.Pawn))
  (Pawn|Input|AddMovementInput (Math|Vector|GetRightVector (Math|Rotator|MakeRotator (.roll _returnvalue_2) (.pitch _returnvalue_2) (.yaw _returnvalue_2))) (.x ActionValue) false)
  (Pawn|Input|AddMovementInput (Math|Vector|GetForwardVector (Math|Rotator|MakeRotator (.roll _returnvalue) (.pitch _returnvalue) (.yaw _returnvalue))) (.y ActionValue) false))

(event Input|EnhancedActionEvents|EnhancedInputActionIA_AttackAction
  (params (ActionValue :type Boolean) (ElapsedSeconds :type Float%20%28double-precision%29) (TriggeredSeconds :type Float%20%28double-precision%29) (InputAction :type Input%20Action%20Object%20Reference :default "/Game/Blueprints/Inputs/IA_AttackAction.IA_AttackAction"))
  (bind _meleepivot (Variables|Default|GetMeleePivot))
  (bind _meleepivot_2 (Variables|Default|GetMeleePivot))
  (bind _returnvalue (Transformation|GetWorldRotation _meleepivot))
  (bind _returnvalue_2 (Transformation|GetWorldRotation _meleepivot_2))
  (:Started
    (Utilities|FlowControl|FlipFlop
      (:A
        (Transformation|SetWorldRotation _meleepivot_2 (Math|Rotator|MakeRotator (.roll _returnvalue_2) (.pitch _returnvalue_2) (- (.yaw _returnvalue_2) 75.0)) false false))
      (:B
        (Transformation|SetWorldRotation _meleepivot (Math|Rotator|MakeRotator (.roll _returnvalue) (.pitch _returnvalue) (- (.yaw _returnvalue) -75.0)) false false)))))

(event EventBeginPlay)

(event EventControllerChanged
  (params (OldController :type Controller%20Object%20Reference) (NewController :type Controller%20Object%20Reference))
  (bind _asplayer_controller (Utilities|Casting|CastToPlayerController NewController))
  (Input|AddMappingContext (PlayerController|LocalPlayerSubsystems|GetEnhancedInputLocalPlayerSubsystem _asplayer_controller) "/Game/Blueprints/Inputs/IMC_Default.IMC_Default" 0 "(bIgnoreAllPressedKeysUntilRelease=True,bForceImmediately=False,bNotifyUserSettings=False)"))

(event EventTick
  (params (DeltaSeconds :type Float%20%28single-precision%29)))

(event Collision|EventActorBeginOverlap
  (params (OtherActor :type Actor%20Object%20Reference)))

(event Input|KeyboardEvents|DebugKey9
  (params (Key :type Key%20Structure :default "None") (ActionValue :type Input%20Action%20Value%20Structure))
  (bind _weaponspawn (Variables|Default|GetWeaponSpawn))
  (bind _returnvalue (Transformation|GetWorldTransform _weaponspawn))
  ;[0.15 0.15 0.15 0.5] Spawn Sword DEBUG
  (:Pressed
    (bind _returnvalue_2 (Game|SpawnActorfromClass "/Game/Blueprints/Weapons/Swords/BP_Sword_Base.BP_Sword_Base_C" (Math|Transform|MakeTransform (Math|Vector|MakeVector (- (.x (.location _returnvalue)) 55.0) (- (.y (.location _returnvalue)) 5e+01) (.z (.location _returnvalue))) (Math|Rotator|MakeRotator (.roll (.rotation _returnvalue)) (.pitch (.rotation _returnvalue)) (+ (.yaw (.rotation _returnvalue)) 45.0)) (.scale _returnvalue)) "Undefined" "MultiplyWithRoot" 0 0))
    (Transformation|AttachComponentToComponent (Variables|/Script/Engine.Actor|GetRootComponent _returnvalue_2) (Variables|Default|GetWeaponSpawn) "None" "KeepRelative" "KeepRelative" "KeepRelative" true)))

(fn ConstructionScript)