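; BP_EnemyBaseProj is an enemy projectile Blueprint that damages the hero on overlap.
; On BeginPlay it waits a tick, plays a fireball sound at its location, and self-destructs after a fixed lifetime.
; Overlapping a BP_Hero_Base sends blockable damage of ProjDmg to that hero's BPCDamageSystem component, then destroys the projectile; other actors are ignored.
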(event EventBeginPlay
  (|CallParentFunction)
  (Utilities|FlowControl|DelayUntilNextTick)
  (Audio|SpawnSoundatLocation "/Game/Audio/SoundCues/SC_Fireball.SC_Fireball" (Transformation|GetWorldLocation (Variables|Default|GetDefaultSceneRoot)) "0, 0, 0" 1.0 1.0 0.0 0 0)
  (Utilities|FlowControl|Delay 15.0)
  (Actor|DestroyActor))

(event Collision|EventActorBeginOverlap
  (params (OtherActor :type Actor%20Object%20Reference))
  (|CallParentFunction OtherActor)
  (bind _asbp_hero_base (Utilities|Casting|CastToBP_Hero_Base OtherActor))
  (Default|TakeDamage (Variables|/Game/Blueprints/Characters/BP_Character_Base.BP_Character_Base_C|GetBPC_DamageSystem _asbp_hero_base) (Utilities|Struct|MakeS_DamageInfo (Variables|Default|GetProjDmg) false true false))
  (Actor|DestroyActor))

(event EventTick
  (params (DeltaSeconds :type Float%20%28single-precision%29))
  (|CallParentFunction DeltaSeconds) ; This node is disabled and will not be called.\nDrag off pins to build functionality.
)

(fn ConstructionScript
  (|CallParentFunction))