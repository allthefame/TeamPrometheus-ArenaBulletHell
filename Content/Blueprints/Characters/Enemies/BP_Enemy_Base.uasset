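; Base enemy character that shoots projectiles at the player hero and deals contact damage through a collision overlap.
; On BeginPlay it caches the hero and binds to its damage component's death event.
; Death awards score to the hero, stops AI logic, plays a sound, drops loot and destroys the actor.
; Loot uses one random roll against cumulative rarity chances, from Common to Legendary or nothing.
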(event OnComponentBeginOverlap(DamageCollision)
  (params (OverlappedComponent :type Primitive%20Component%20Object%20Reference) (OtherActor :type Actor%20Object%20Reference) (OtherComp :type Primitive%20Component%20Object%20Reference) (OtherBodyIndex :type Integer) (bFromSweep :type Boolean) (SweepResult :type Hit%20Result%20Structure%20%28by%20ref%29))
  ;[0.15 0.003691 0 0.5] Enemy Damage
  (bind _asbp_hero_base (Utilities|Casting|CastToBP_Hero_Base OtherActor))
  (Default|TakeDamage (Variables|/Game/Blueprints/Characters/BP_Character_Base.BP_Character_Base_C|GetBPC_DamageSystem _asbp_hero_base) (Utilities|Struct|MakeS_DamageInfo 1.0 "NewEnumerator0")))

(event Custom|SimpleAttack
  ;[0.09427 0.01015 0.15 0.5] Fire projectiles toward player
  (Audio|SpawnSoundatLocation "/Game/Audio/Ref/Monster_Grunt_Shortened_V_5.Monster_Grunt_Shortened_V_5" (Transformation|GetWorldLocation (Variables|Default|GetCapsuleComponent)) "0, 0, 0" 1.0 1.0 0.0 0 0)
  (Game|SpawnActorfromClass "/Game/Blueprints/Weapons/Projectiles/BP_EnemyBaseProj.BP_EnemyBaseProj_C" (Math|Transform|MakeTransform (.location (Transformation|GetWorldTransform (Variables|Default|GetCapsuleComponent))) (Math|Conversions|RotationFromXVector (Math|Vector|GetUnitDirection(Vector) (Transformation|GetWorldLocation (Variables|Default|GetCapsuleComponent)) (Transformation|GetWorldLocation (Variables|/Script/Engine.Character|GetCapsuleComponent (Variables|Default|GetPlayerRef))))) "1.000000,1.000000,1.000000") "Undefined" "MultiplyWithRoot" 0 0))

(event Custom|OnDeathEvent
  ;[0.03399 0.15 0 0.5] Comment
  (Default|OnEnemyKilledEvent (Variables|Default|GetPlayerRef) (Variables|Default|GetEnemyScoreGain))
  (AI|Logic|StopLogic (Variables|/Script/AIModule.AIController|GetBrainComponent (AI|GetAIController self)) "")
  (Audio|SpawnSoundatLocation "/Game/Audio/Ref/Monster_Grrr_Shortened_V_2.Monster_Grrr_Shortened_V_2" (Transformation|GetWorldLocation (Variables|Default|GetCapsuleComponent)) "0, 0, 0" 1.0 1.0 0.0 0 0)
  (CallFunction|GetTieredDrop)
  (Actor|DestroyActor))

(event Custom|GetTieredDrop
  ;[0.15 0.15 0.15 0.5] Drop Item Based On Rarity (Common + Uncommon + Rare + Epic + Legendary <= 100)
  (bind _output_get (Variables|Default|SetRandIntForItem (Math|Random|RandomIntegerinRange 1 100)))
  (Development|PrintString (Utilities|String|ToString(Integer) _output_get) true true "(R=0.000000,G=0.660000,B=1.000000,A=1.000000)" 6.0)
  (if (<= _output_get (Variables|Default|GetProbCommon))
    (Game|SpawnActorfromClass "/Game/Blueprints/Items/LootBags/BP_Item_Common.BP_Item_Common_C" (Transformation|GetActorTransform self) "Undefined" "MultiplyWithRoot" 0 0 0)
    (Development|PrintString "Common")
    (elif (<= _output_get (+ (Variables|Default|GetProbCommon) (Variables|Default|GetProbUnCommon)))
      (Game|SpawnActorfromClass "/Game/Blueprints/Items/LootBags/BP_Item_Uncommon.BP_Item_Uncommon_C" (Transformation|GetActorTransform self) "Undefined" "MultiplyWithRoot" 0 0 0)
      (Development|PrintString "Uncommon")
      (elif (<= _output_get (+ (Variables|Default|GetProbCommon) (Variables|Default|GetProbUnCommon) (Variables|Default|GetProbRare)))
        (Game|SpawnActorfromClass "/Game/Blueprints/Items/LootBags/BP_Item_Rare.BP_Item_Rare_C" (Transformation|GetActorTransform self) "Undefined" "MultiplyWithRoot" 0 0 0)
        (Development|PrintString "Rare")
        (elif (<= _output_get (+ (Variables|Default|GetProbCommon) (Variables|Default|GetProbUnCommon) (Variables|Default|GetProbRare) (Variables|Default|GetProbEpic)))
          (Game|SpawnActorfromClass "/Game/Blueprints/Items/LootBags/BP_Item_Epic.BP_Item_Epic_C" (Transformation|GetActorTransform self) "Undefined" "MultiplyWithRoot" 0 0 0)
          (Development|PrintString "Epic")
          (elif (<= _output_get (+ (Variables|Default|GetProbCommon) (Variables|Default|GetProbUnCommon) (Variables|Default|GetProbRare) (Variables|Default|GetProbEpic) (Variables|Default|GetProbLegendary)))
            (Game|SpawnActorfromClass "/Game/Blueprints/Items/LootBags/BP_Item_Legendary.BP_Item_Legendary_C" (Transformation|GetActorTransform self) "Undefined" "MultiplyWithRoot" 0 0 0)
            (Development|PrintString "Lengendary")
            (else
              (Development|PrintString "Drop Nothing"))))))))

(event EventBeginPlay
  ;[0.03399 0.15 0 0.5] Comment
  (|CallParentFunction)
  (bind _asbp_hero_base (Utilities|Casting|CastToBP_Hero_Base (Game|GetPlayerCharacter 0)))
  (Variables|Default|SetPlayerRef _asbp_hero_base)
  (EventDispatchers|AssignOnDeath (Variables|Default|GetBPC_DamageSystem) (delegate Custom|OnDeathEvent)))

(fn ConstructionScript
  (|CallParentFunction))

(fn GetReference
  (return self))