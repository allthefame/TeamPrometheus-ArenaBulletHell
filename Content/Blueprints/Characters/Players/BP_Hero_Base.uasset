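; Base player hero with a flipping sprite, Enhanced Input movement and a cooldown-limited projectile aimed at the cursor.
; BPCDamageSystem gates movement and attacks; its death event plays a sound, stops enemy AI and shows the death screen.
; Event dispatchers drive looping footstep start/stop and score accumulation from kills.
; Also creates the HUD, forces windowed fullscreen, toggles the pause menu and includes debug keys for health, damage and inventory tracing.
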(event Custom|OnDeathEvent
  ;[0 0.1231 0.15 0.5] On Death Event
  (Development|PrintString "Player is Dead")
  (Audio|SpawnSoundatLocation "/Game/Audio/Ref/Death_Sound.Death_Sound" (Transformation|GetWorldLocation (Variables|Default|GetCapsuleComponent)) "0, 0, 0" 1.0 1.0 0.0 0 0)
  ;;[0.15 0.15 0.15 0.5] Enemies stop moving
  (bind _outactors (Actor|GetAllActorsOfClass "/Game/Blueprints/Characters/Enemies/BP_Enemy_Base.BP_Enemy_Base_C"))
  (for _array_element _outactors
    (AI|Logic|StopLogic (Variables|/Script/AIModule.AIController|GetBrainComponent (AI|GetAIController _array_element)) ""))
  (Viewport|RemoveAllWidgets)
  (bind _returnvalue (UserInterface|CreateWidget "/Game/Blueprints/Widgets/WBP_DeathScreen.WBP_DeathScreen_C"))
  (UserInterface|Viewport|AddtoViewport _returnvalue 0))

(event Custom|IsWalkingEvent
  (params (IsWalking :type Boolean))
  ;[0.15 0.000763 0.09471 0.5] Footsteps Audio
  (if (Variables|/Game/Blueprints/Components/BPC_DamageSystem.BPC_DamageSystem_C|GetIsDead (Variables|Default|GetBPC_DamageSystem))
    (Audio|Components|Audio|Stop (Variables|Default|GetFootstepsSound) :!label _label)
    (elif IsWalking
      (bind _returnvalue (Audio|CreateSound2D "/Game/Audio/SoundCues/SC_Steps.SC_Steps" 1.0 1.0 0.0 0 false false))
      (bind _output_get (Variables|Default|SetFootstepsSound _returnvalue))
      (Audio|Components|Audio|Play _output_get 0.0)
      (else
        (goto _label)))))

(event Custom|OnEnemyKilledEvent
  (params (ScoreToAdd :type Integer))
  ;[0.15 0.04953 0 0.5] Scoring
  (bind _output_get (Variables|Default|SetScore (+ ScoreToAdd (Variables|Default|GetScore)))))

(event Custom|FlipSprite
  (params (ActionValueX :type Float%20%28double-precision%29))
  ;[0.15 0.15 0.15 0.5] Handle Flip Sprite
  (if (> ActionValueX 0.0)
    (Transformation|SetRelativeRotation (Variables|Default|GetSprite) "0.000000,90.000000,-90.000000" false false)
    (elif (< ActionValueX 0.0)
      (Transformation|SetRelativeRotation (Variables|Default|GetSprite) "180.000000,90.000000,-90.000000" false false))))

(event Input|EnhancedActionEvents|EnhancedInputActionIA_Move
  (params (ActionValue :type Vector%202D%20Structure) (ElapsedSeconds :type Float%20%28double-precision%29) (TriggeredSeconds :type Float%20%28double-precision%29) (InputAction :type Input%20Action%20Object%20Reference :default "/Game/Blueprints/Inputs/IA_Move.IA_Move"))
  (bind _returnvalue (Pawn|GetControlRotation :!class /Script/Engine.Pawn))
  (bind _returnvalue_2 (Pawn|GetControlRotation :!class /Script/Engine.Pawn))
  ;[0 0.15 0.06616 0.5] Player Movement
  (:Triggered
    (if (not (Variables|/Game/Blueprints/Components/BPC_DamageSystem.BPC_DamageSystem_C|GetIsDead (Variables|Default|GetBPC_DamageSystem)))
      (Pawn|Input|AddMovementInput (Math|Vector|GetRightVector (Math|Rotator|MakeRotator (.roll _returnvalue_2) (.pitch _returnvalue_2) (.yaw _returnvalue_2))) (.x ActionValue) false)
      (Pawn|Input|AddMovementInput (Math|Vector|GetForwardVector (Math|Rotator|MakeRotator (.roll _returnvalue) (.pitch _returnvalue) (.yaw _returnvalue))) (.y ActionValue) false)
      (CallFunction|FlipSprite (.x ActionValue))))
  (:Started
    (Default|CallIsWalkingforFootsteps true))
  (:Completed
    (Default|CallIsWalkingforFootsteps false)))

(event Input|EnhancedActionEvents|EnhancedInputActionIA_AttackAction
  (params (ActionValue :type Boolean) (ElapsedSeconds :type Float%20%28double-precision%29) (TriggeredSeconds :type Float%20%28double-precision%29) (InputAction :type Input%20Action%20Object%20Reference :default "/Game/Blueprints/Inputs/IA_AttackAction.IA_AttackAction"))
  ;[1 1 1 0.5] Extras??
)

(event Input|EnhancedActionEvents|EnhancedInputActionIA_AttackAction
  (params (ActionValue :type Boolean) (ElapsedSeconds :type Float%20%28double-precision%29) (TriggeredSeconds :type Float%20%28double-precision%29) (InputAction :type Input%20Action%20Object%20Reference :default "/Game/Blueprints/Inputs/IA_AttackAction.IA_AttackAction"))
  (bind _returnvalue (Transformation|GetActorLocation))
  ;[0 0.02236 0.15 0.5] Basic Projectile
  (if (not (Variables|/Game/Blueprints/Components/BPC_DamageSystem.BPC_DamageSystem_C|GetIsDead (Variables|Default|GetBPC_DamageSystem)))
    (if (not (Variables|Default|GetAttackOnCooldown))
      (Game|SpawnActorfromClass "/Game/Blueprints/Weapons/Projectiles/BP_HeroBaseProj.BP_HeroBaseProj_C" (Math|Transform|MakeTransform (Math|Vector|MakeVector (.x _returnvalue) (.y _returnvalue) (.z _returnvalue)) (Math|Rotator|MakeRotator 0.0 0.0 (.yaw (Math|Rotator|FindLookatRotation (Math|Vector|MakeVector (.x _returnvalue) (.y _returnvalue) 0.0) (.Location (Collision|BreakHitResult (.HitResult (Game|Player|GetHitResultUnderCursorbyChannel (Game|GetPlayerController 0) "TraceTypeQuery1" true))))))) "1.000000,1.000000,1.000000") "Undefined" "MultiplyWithRoot" 0 0)
      (Variables|Default|SetAttackOnCooldown true)
      (Utilities|FlowControl|Delay (Variables|Default|GetAttackCooldownDuration))
      (Variables|Default|SetAttackOnCooldown false))))

(event Input|EnhancedActionEvents|EnhancedInputActionIA_Pause
  (params (ActionValue :type Boolean) (ElapsedSeconds :type Float%20%28double-precision%29) (TriggeredSeconds :type Float%20%28double-precision%29) (InputAction :type Input%20Action%20Object%20Reference :default "/Game/Blueprints/Inputs/IA_Pause.IA_Pause"))
  (bind _returnvalue (Game|GetPlayerController 0))
  ;[0.3031 0.2105 0.04452 0.5] Pausing the Game
  (:Started
    (if (Variables|Default|GetPaused?)
      (Variables|Default|SetPaused? false)
      (Widget|RemovefromParent (stale _returnvalue_2))
      (Game|SetGamePaused false)
      (else
        (Variables|Default|SetPaused? true)
        (bind _returnvalue_2 (UserInterface|CreateWidget "/Game/Blueprints/Widgets/GameScreens/WBP_PauseMenu.WBP_PauseMenu_C"))
        (UserInterface|Viewport|AddtoViewport _returnvalue_2 0)
        (Variables|/Script/Engine.PlayerController|SetbShowMouseCursor _returnvalue true)
        (Input|SetInputModeGameandUI _returnvalue 0 "DoNotLock" false false)
        (Game|SetGamePaused true)))))

(event EventBeginPlay
  ;[0 0 0 0.5] Beginning Sequence
  (|CallParentFunction)
  (Utilities|FlowControl|Sequence
    (:then_0
      ;[0 0.1231 0.15 0.5] On Death Event
      (EventDispatchers|BindEventtoOnDeath (Variables|Default|GetBPC_DamageSystem) (delegate Custom|OnDeathEvent)))
    (:then_1
      ;[0.15 0.000763 0.09471 0.5] Footsteps Audio
      (EventDispatchers|BindEventtoIsWalkingforFootsteps (delegate Custom|IsWalkingEvent)))
    (:then_2
      ;[0.15 0.04953 0 0.5] Scoring
      (EventDispatchers|BindEventtoOnEnemyKilled (delegate Custom|OnEnemyKilledEvent)))
    (:then_3
      ;[0.04494 0.15 0 0.5] Fullscreen Changes
      (bind _returnvalue (Settings|GetGameUserSettings))
      (Class|GameUserSettings|SetFullscreenMode _returnvalue "WindowedFullscreen")
      (Class|GameUserSettings|ApplySettings _returnvalue true))
    (:then_4
      ;[0.15 0.07914 0.145 0.5] Add HUD to Viewport
      (bind _returnvalue_2 (UserInterface|CreateWidget "/Game/Blueprints/Widgets/WBP_HUD.WBP_HUD_C"))
      (UserInterface|Viewport|AddtoViewport _returnvalue_2 0))))

(event EventControllerChanged
  (params (OldController :type Controller%20Object%20Reference) (NewController :type Controller%20Object%20Reference))
  ;[0 0.15 0.06616 0.5] Player Movement
  (bind _asplayer_controller (Utilities|Casting|CastToPlayerController NewController))
  (Input|AddMappingContext (PlayerController|LocalPlayerSubsystems|GetEnhancedInputLocalPlayerSubsystem _asplayer_controller) "/Game/Blueprints/Inputs/IMC_Default.IMC_Default" 0 "(bIgnoreAllPressedKeysUntilRelease=True,bForceImmediately=False,bNotifyUserSettings=False)"))

(event EventTick
  (params (DeltaSeconds :type Float%20%28single-precision%29))
  ;[1 1 1 0.5] Extras??
  (|CallParentFunction DeltaSeconds))

(event Collision|EventActorBeginOverlap
  (params (OtherActor :type Actor%20Object%20Reference))
  ;[1 1 1 0.5] Extras??
  (|CallParentFunction OtherActor))

(event Input|KeyboardEvents|DebugKey9
  (params (Key :type Key%20Structure :default "None") (ActionValue :type Input%20Action%20Value%20Structure))
  ;[0.3932 0.1649 0.1649 0.5] Spawn Sword DEBUG, ARCHIVED
)

(event Input|KeyboardEvents|DebugKeyH
  (params (Key :type Key%20Structure :default "None") (ActionValue :type Input%20Action%20Value%20Structure))
  (bind _bpc_damagesystem (Variables|Default|GetBPC_DamageSystem))
  ;[0.1386 0.15 0.003923 0.5] Damage System Proof DEBUG
  (:Pressed
    (Development|PrintString (Utilities|String|ToString(Text) (Utilities|Text|FormatText "Player Health: {CurHealth}/{MaxHealth}" (Variables|/Game/Blueprints/Components/BPC_DamageSystem.BPC_DamageSystem_C|GetCurHealth _bpc_damagesystem) (Variables|/Game/Blueprints/Components/BPC_DamageSystem.BPC_DamageSystem_C|GetMaxHealth _bpc_damagesystem))))))

(event Input|KeyboardEvents|DebugKeyJ
  (params (Key :type Key%20Structure :default "None") (ActionValue :type Input%20Action%20Value%20Structure))
  ;[0.1386 0.15 0.003923 0.5] Damage System Proof DEBUG
  (:Pressed
    (bind _wasdamaged (Default|TakeDamage (Variables|Default|GetBPC_DamageSystem) (Utilities|Struct|MakeS_DamageInfo 1.0 "NewEnumerator0")))
    (if _wasdamaged
      (Development|PrintString "Player was dealt 1 damage =-(")
      (else
        (Development|PrintString "Player is DEAD X-P")))))

(event Input|KeyboardEvents|DebugKeyF
  (params (Key :type Key%20Structure :default "None") (ActionValue :type Input%20Action%20Value%20Structure))
  ;[1 1 1 0.5] Extras??
  (:Pressed
    (Default|TraceInteractableObjects (Variables|Default|GetBPC_SpatialInventory))))

(fn ConstructionScript
  (|CallParentFunction))