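; BP_ContainerItem is an item definition for the spatial inventory, exposing name, dimensions, thumbnails, container rows, slot type, actions, placeholder flag and the actor to spawn.
; Rotate toggles a flag that makes GetDimensions swap X and Y and GetThumbnail return the rotated image.
; Both thumbnail getters fall back to M_Null for invalid assets; the main one requires both orientations to be valid.
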(fn GetRows
  (return (Variables|Default|GetContainerRows)))

(fn GetName
  (return (Variables|Default|GetName)))

(fn GetThumbnail
  ;[0.15 0.15 0.15 0.5] ContainerItem
  (if (and (Utilities|IsValid (Variables|Default|GetThumbnail)) (Utilities|IsValid (Variables|Default|GetThumbnailRotated)))
    (if (Variables|Default|GetRotated)
      (return (Variables|Default|GetThumbnailRotated))
      (else
        (return (Variables|Default|GetThumbnail))))
    (else
      (return "/Game/Art/UI/M_Null.M_Null"))))

(fn GetDimensions
  (bind _dimension (Variables|Default|GetDimension))
  (if (Variables|Default|GetRotated)
    (return (Utilities|Struct|MakeIntPoint (.y _dimension) (.x _dimension)))
    (else
      (return (Variables|Default|GetDimension)))))

(fn Rotate
  (Variables|Default|SetRotated (not (Variables|Default|GetRotated)))
  (return))

(fn GetActortoSpawn
  (return (Variables|Default|GetActorToSpawn)))

(fn GetActions
  (return (Variables|Default|GetActions)))

(fn GetContainerSlotType
  (return (Variables|Default|GetContainerSlotType)))

(fn GetIsPlaceholder
  (return (Variables|Default|GetIsPlaceholder)))

(fn GetSquareThumbnail
  (if (Utilities|IsValid (Variables|Default|GetSquareThumbnail))
    (return (Variables|Default|GetSquareThumbnail))
    (else
      (return "/Game/Art/UI/M_Null.M_Null"))))