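; BP_ContainerCell is a data holder for a cell container in the spatial inventory system, storing Dimensions, a Usable value and an Items array.
; Getters expose all three values, while SetItemAtIndex writes an item into a given array slot.
; RemoveItemAtIndex overwrites the slot with an empty default instead of deleting the element, so the indices of other items stay fixed.
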(fn GetDimensions
  (return (Variables|Default|GetDimensions)))

(fn GetUsable
  (return (Variables|Default|GetUsable)))

(fn GetItems
  (return (Variables|Default|GetItems)))

(fn SetItematIndex
  (params (Item :type BP%20Container%20Item%20Object%20Reference) (Index :type Integer))
  (Utilities|Array|SetArrayElem (Variables|Default|GetItems) Index Item))

(fn RemoveItematIndex
  (params (Index :type Integer))
  (Utilities|Array|SetArrayElem (Variables|Default|GetItems) Index 0))