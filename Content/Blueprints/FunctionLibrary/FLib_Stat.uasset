(fn GetSubStatIdx
  (params (MainStat :type S%20Main%20Stat%20Structure) (SubStatType :type Enum_SubStatType%20Enum :default "NewEnumerator0"))
  (for (_array_element _array_index) (Utilities|Struct|BreakS_MainStat MainStat)
    (LocalVariables|SetTargetIdx _array_index)
    (if (Utilities|Enum|Equal(Enum) (Utilities|Struct|BreakS_SubStat _array_element) SubStatType)
      (return (LocalVariables|GetTargetIdx) true)))
  (Development|PrintString 0 (Utilities|String|Append "Didn't find \"" (Utilities|String|EnumtoString SubStatType) "\" in  " (Utilities|String|EnumtoString (Utilities|Struct|BreakS_MainStat MainStat))))
  (return -1 false))

(fn CreateMainStat
  (params (Name :type String) (MainStatType :type Enum_MainStatType%20Enum :default "NewEnumerator4") (PointsToUnlockSub :type Integer))
  (return (Utilities|Struct|MakeS_MainStat Name 0 MainStatType PointsToUnlockSub)))

(fn AddSubStat
  (params (TargetMainStat :type S%20Main%20Stat%20Structure%20%28by%20ref%29) (SubStatName :type String) (SubStatType :type Enum_SubStatType%20Enum :default "NewEnumerator20") (PointsToUnlockTer :type Integer))
  (for _array_element (Utilities|Struct|BreakS_MainStat TargetMainStat)
    (if (Utilities|Enum|Equal(Enum) (Utilities|Struct|BreakS_SubStat _array_element) SubStatType)
      (Development|PrintString 0 (Utilities|String|Append "Add SubStat Failed! " (Utilities|String|EnumtoString SubStatType) " is already in " (Utilities|String|EnumtoString (Utilities|Struct|BreakS_MainStat TargetMainStat))) true true "(R=1.000000,G=0.041141,B=0.031194,A=1.000000)" 6.0)
      (return false)))
  (bind _newsubstat (CallFunction|CreateSubStat SubStatName SubStatType PointsToUnlockTer))
  (Utilities|Array|Add (Utilities|Struct|BreakS_MainStat TargetMainStat) _newsubstat)
  (Development|PrintString 0 (Utilities|String|Append "Add " (Utilities|String|EnumtoString SubStatType) " to " (Utilities|String|EnumtoString (Utilities|Struct|BreakS_MainStat TargetMainStat)) " Successfully!") true true "(R=0.133703,G=0.807292,B=0.001183,A=1.000000)" 6.0)
  (return true))

(fn CreateSubStat
  (params (Name :type String) (SubStatType :type Enum_SubStatType%20Enum :default "NewEnumerator20") (PointsToUnlockTer :type Integer))
  (return (Utilities|Struct|MakeS_SubStat Name SubStatType PointsToUnlockTer)))

(fn CreateTerStat
  (params (Name :type String) (TerStatType :type Enum_TertiaryStatType%20Enum :default "NewEnumerator0"))
  (return (Utilities|Struct|MakeS_TertiaryStat Name TerStatType)))

(fn AddTerStat
  (params (TargetSubStat :type S%20Sub%20Stat%20Structure%20%28by%20ref%29) (TerStatName :type String%20%28by%20ref%29) (TerStatType :type Enum_TertiaryStatType%20Enum%20%28by%20ref%29 :default "NewEnumerator0"))
  (for _array_element (Utilities|Struct|BreakS_SubStat TargetSubStat)
    (if (Utilities|Enum|Equal(Enum) (Utilities|Struct|BreakS_TertiaryStat _array_element) TerStatType)
      (Development|PrintString 0 (Utilities|String|Append "Add TerStat Failed! " (Utilities|String|EnumtoString TerStatType) " is already in " (Utilities|String|EnumtoString (Utilities|Struct|BreakS_SubStat TargetSubStat))))
      (return false)))
  (bind _newterstat (CallFunction|CreateTerStat TerStatName TerStatType))
  (Utilities|Array|Add (Utilities|Struct|BreakS_SubStat TargetSubStat) _newterstat)
  (Development|PrintString 0 (Utilities|String|Append "Add " (Utilities|String|EnumtoString TerStatType) " to " (Utilities|String|EnumtoString (Utilities|Struct|BreakS_SubStat TargetSubStat)) " Successfully!") true true "(R=0.174475,G=0.177083,B=0.175127,A=1.000000)" 5.0)
  (return true))