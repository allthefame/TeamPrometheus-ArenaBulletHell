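; Base enemy projectile Blueprint that damages the player's hero on overlap.
; On spawn it waits one tick, plays a fireball sound at its location, then destroys itself after a fixed lifetime.
; Overlapping a BP_Hero_Base sends ProjDmg through the hero's BPCDamageSystem component and destroys the projectile, while other actors are ignored.
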(event EventBeginPlay
  ;[0.8125 0.003609 0 0.5] Enemy Damage Projectile
  (|CallParentFunction)
  (Utilities|FlowControl|DelayUntilNextTick)
  (Audio|SpawnSoundatLocation "/Game/Audio/SoundCues/SC_RandomFireballs.SC_RandomFireballs" (Transformation|GetWorldLocation (Variables|Default|GetDefaultSceneRoot)) "0, 0, 0" 1.0 1.0 0.0 0 0)
  (Utilities|FlowControl|Delay 15.0)
  (Actor|DestroyActor))

(event Collision|EventActorBeginOverlap
  (params (OtherActor :type Actor%20Object%20Reference))
  ;[0.8125 0.003609 0 0.5] Enemy Damage Projectile
  (|CallParentFunction OtherActor)
  (bind _asbp_hero_base (Utilities|Casting|CastToBP_Hero_Base OtherActor))
  (Default|TakeDamage (Variables|/Game/Blueprints/Characters/BP_Character_Base.BP_Character_Base_C|GetBPC_DamageSystem _asbp_hero_base) (Utilities|Struct|MakeS_DamageInfo (Variables|Default|GetProjDmg) "NewEnumerator0" true))
  (Actor|DestroyActor))

(event EventTick
  (params (DeltaSeconds :type Float%20%28single-precision%29))
  (|CallParentFunction DeltaSeconds) ; This node is disabled and will not be called.\nDrag off pins to build functionality.
)

(fn ConstructionScript
  (|CallParentFunction))