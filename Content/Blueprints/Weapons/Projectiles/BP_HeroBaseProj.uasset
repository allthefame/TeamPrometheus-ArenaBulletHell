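; Base hero projectile actor, apparently a sword, that damages enemies it touches.
; On BeginPlay it waits a tick, plays a sword sound at its location and destroys itself after a fixed lifetime.
; Overlapping a BP_Enemy_Base sends blockable ProjDmg plus a map of effect values to that enemy's BPCDamageSystem, then destroys the projectile; other actors are ignored.
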(event EventBeginPlay
  ;[0.04138 0.1478 0.15 0.5] Sword Activation
  (|CallParentFunction)
  (Utilities|FlowControl|DelayUntilNextTick)
  (Audio|SpawnSoundatLocation "/Game/Audio/SoundCues/SC_RandomSwords.SC_RandomSwords" (Transformation|GetWorldLocation (Variables|Default|GetDefaultSceneRoot)) "0, 0, 0" 1.0 1.0 0.0 0 0)
  (Utilities|FlowControl|Delay 15.0)
  (Actor|DestroyActor))

(event Collision|EventActorBeginOverlap
  (params (OtherActor :type Actor%20Object%20Reference))
  ;[0.1478 0.15 0.03041 0.5] Sword Damage
  (|CallParentFunction OtherActor)
  (bind _asbp_enemy_base (Utilities|Casting|CastToBP_Enemy_Base OtherActor))
  (Default|TakeDamage (Variables|/Game/Blueprints/Characters/BP_Character_Base.BP_Character_Base_C|GetBPC_DamageSystem _asbp_enemy_base) (Utilities|Struct|MakeS_DamageInfo (Variables|Default|GetProjDmg) "NewEnumerator0" true false (Utilities|Struct|MakeS_DamageEffects (Utilities|Map|MakeMap "NewEnumerator1" 3 "NewEnumerator2" 5 "NewEnumerator4" 2))))
  (Actor|DestroyActor))

(event EventTick
  (params (DeltaSeconds :type Float%20%28single-precision%29))
  (|CallParentFunction DeltaSeconds) ; This node is disabled and will not be called.\nDrag off pins to build functionality.
)

(fn ConstructionScript
  (|CallParentFunction))