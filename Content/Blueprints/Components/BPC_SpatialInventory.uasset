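; Hero inventory component for a Tarkov-style spatial grid, with pickup, drop, secret pouch equipping and a toggleable UI widget.
; Container items hold rows of cells, each a flattened 2D array where items fill every index they cover; searches recurse into nested containers.
; Sphere-traced pickups take the first free space in equipped slots, retrying rotated.
; Item changes fire an update call, and drops spawn the item's actor at the hero.
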(event Custom|AddItemToInventory
  (params (Cell :type BP%20Container%20Cell%20Object%20Reference) (Item :type BP%20Container%20Item%20Object%20Reference) (Index :type Integer))
  (CallFunction|AddItemtoContainer Cell Item Index))

(event Custom|ToggleInventoryVisibility
  (bind _inventorywidget (Variables|UI|GetInventoryWidget)
    (:then
      (Widget|RemovefromParent _inventorywidget)
      (Variables|UI|SetInventoryWidget 0)
      (Input|SetInputModeGameOnly (Game|GetPlayerController 0) false))
    (:else
      (bind _returnvalue (UserInterface|CreateWidget "/Game/Blueprints/Widgets/WBP_SpatialInventory.WBP_SpatialInventory_C" 0 self))
      (bind _output_get (Variables|UI|SetInventoryWidget _returnvalue))
      (UserInterface|Viewport|AddtoViewport _output_get 0)
      (Input|SetInputModeUIOnly (Game|GetPlayerController 0) 0 "DoNotLock" false))))

(event Custom|HandleActionForItems
  (params (Action :type Enum_ContainerItemActions%20Enum :default "NewEnumerator0") (Item :type BP%20Container%20Item%20Object%20Reference))
  (bind (_cell _container _index _result) (CallFunction|FindItem Item))
  (if _result
    (CallFunction|HandleContainerItemAction Action Item _cell)))

(event Input|EnhancedActionEvents|EnhancedInputActionIA_Inventory
  (params (ActionValue :type Boolean) (ElapsedSeconds :type Float%20%28double-precision%29) (TriggeredSeconds :type Float%20%28double-precision%29) (InputAction :type Input%20Action%20Object%20Reference :default "/Game/Blueprints/Inputs/IA_Inventory.IA_Inventory"))
  (:Started
    (CallFunction|ToggleInventoryVisibility)))

(event EventBeginPlay
  (CallFunction|Initialize))

(fn Initialize
  (bind _defaultcontainerdimensions (Variables|Default|GetDefaultContainerDimensions))
  (bind _asbp_hero_base (Utilities|Casting|CastToBP_Hero_Base (Components|GetOwner)))
  (Variables|Default|SetHeroRef _asbp_hero_base)
  (Utilities|FlowControl|Sequence
    (:then_0
      ;[0 0.08493 1 0.5] Make Base Inventory Grid
      (Utilities|Array|Resize (LocalVariables|GetLocalDefaultContainerItems) (* (.x _defaultcontainerdimensions) (.y _defaultcontainerdimensions)))
      (bind _returnvalue (Game|ConstructObjectfromClass "/Game/Blueprints/SpatialInventory/BP_ContainerCell.BP_ContainerCell_C" (Variables|Default|GetDefaultContainerDimensions) true (LocalVariables|GetLocalDefaultContainerItems)))
      (bind _returnvalue_2 (Game|ConstructObjectfromClass "/Game/Blueprints/SpatialInventory/BP_ContainerItem.BP_ContainerItem_C" (Utilities|Struct|MakeIntPoint 10 5) "" 0 0 (Utilities|Array|MakeArray (Utilities|Struct|MakeS_ContainerRow (Utilities|Array|MakeArray _returnvalue))) false 0 "(INVALID)" 0))
      (Variables|Slots|SetSecretPocketSlot _returnvalue_2))))

(fn GetAllContainerItems
  ;[0.15 0.15 0.15 0.5] Looks for all the items in the inventory and returns them
  (for _array_element (Slots|GetAllSlots)
    (Utilities|Array|Add (LocalVariables|GetLocalContainerItems) _array_element)
    (bind _items (CallFunction|GetItemsfromItem _array_element))
    (for _array_element_2 _items
      (if (Utilities|Array|IsNotEmpty (Default|GetRows _array_element_2))
        (Utilities|Array|Add (LocalVariables|GetLocalContainerItems) _array_element_2))))
  (return (LocalVariables|GetLocalContainerItems)))

(fn CanAddItemtoInventory
  (params (ItemToAdd :type BP%20Container%20Item%20Object%20Reference))
  (for _array_element (Slots|GetAllSlots)
    (bind (_cell _index _result) (CallFunction|HasPlaceforIteminContainer ItemToAdd _array_element))
    (if _result
      (return _array_element _cell _index _result)))
  (return 0 0 0 false))

(fn HasPlaceforIteminContainer
  (params (Item :type BP%20Container%20Item%20Object%20Reference) (Container :type BP%20Container%20Item%20Object%20Reference))
  (for _array_element (Default|GetRows Container)
    (for _array_element_2 (Utilities|Struct|BreakS_ContainerRow _array_element)
      (bind (_x _y _result) (CallFunction|HasPlaceforIteminCell Item _array_element_2))
      (if _result
        (return _array_element_2 (+ _x (* _y (.x (Default|GetDimensions _array_element_2)))) true))))
  (return 0 0 false))

(fn HasPlaceforIteminCell
  (params (Item :type BP%20Container%20Item%20Object%20Reference) (Cell :type BP%20Container%20Cell%20Object%20Reference))
  (bind _dimension (Default|GetDimensions Item))
  (bind _dimensions (Default|GetDimensions Cell))
  (bind _dimensions_2 (Default|GetDimensions Cell))
  (bind (_x _y) (Utilities|Struct|BreakIntPoint _dimensions_2))
  (if (and (>= (.x _dimensions) (.x _dimension)) (>= (.y _dimensions) (.y _dimension)))
    (for _index (range 0 (- _y 1))
      (LocalVariables|SetLocalY _index)
      (for _index_2 (range 0 (- _x 1))
        (LocalVariables|SetLocalX _index_2)
        (LocalVariables|SetLocalValid true)
        (bind (_x_2 _y_2 _result) (CallFunction|CanStoreIteminCellatLocation Cell Item (LocalVariables|GetLocalX) (LocalVariables|GetLocalY)))
        (if _result
          (return _x_2 _y_2 true))))
    (return 0 0 false)
    (else
      (return 0 0 false))))

(fn AddItemtoContainer
  (params (Cell :type BP%20Container%20Cell%20Object%20Reference) (Item :type BP%20Container%20Item%20Object%20Reference) (Index :type Integer))
  (bind _dimensions (Default|GetDimensions Cell))
  (CallFunction|AddItemtoCellatLocation Cell Item (Utilities|Struct|MakeIntPoint (Math|Integer|%(Integer) Index (.x _dimensions)) (/ Index (.y _dimensions)))))

(fn TraceInteractableObjects
  (bind _heroref (Variables|Default|GetHeroRef))
  (bind _capsulecomponent (Variables|/Script/Engine.Character|GetCapsuleComponent _heroref))
  (bind _returnvalue (Transformation|GetWorldLocation _capsulecomponent))
  (bind (_outhit _returnvalue_2) (Collision|SphereTraceByChannel _returnvalue _returnvalue 2e+02 "TraceTypeQuery1" false 0 "ForDuration"))
  (if _returnvalue_2
    (Utilities|IsValid (.HitActor (Collision|BreakHitResult _outhit))
      (:Is%20Valid
        (Utilities|IsValid (Actor|GetComponentbyClass (.HitActor (Collision|BreakHitResult _outhit)) "/Game/Blueprints/Components/BPC_InteractableObject.BPC_InteractableObject_C")
          (:Is%20Valid
            (bind (_container _cell _index _result) (CallFunction|CanAddItemtoInventory (Variables|/Game/Blueprints/Components/BPC_InteractableObject.BPC_InteractableObject_C|GetItem (Actor|GetComponentbyClass (.HitActor (Collision|BreakHitResult _outhit)) "/Game/Blueprints/Components/BPC_InteractableObject.BPC_InteractableObject_C"))))
            (if _result
              (CallFunction|AddItemtoInventory _cell (Variables|/Game/Blueprints/Components/BPC_InteractableObject.BPC_InteractableObject_C|GetItem (Actor|GetComponentbyClass (.HitActor (Collision|BreakHitResult _outhit)) "/Game/Blueprints/Components/BPC_InteractableObject.BPC_InteractableObject_C")) _index)
              (Actor|DestroyActor (.HitActor (Collision|BreakHitResult _outhit)))
              (else
                (Default|Rotate (Variables|/Game/Blueprints/Components/BPC_InteractableObject.BPC_InteractableObject_C|GetItem (Actor|GetComponentbyClass (.HitActor (Collision|BreakHitResult _outhit)) "/Game/Blueprints/Components/BPC_InteractableObject.BPC_InteractableObject_C")))
                (bind (_container_2 _cell_2 _index_2 _result_2) (CallFunction|CanAddItemtoInventory (Variables|/Game/Blueprints/Components/BPC_InteractableObject.BPC_InteractableObject_C|GetItem (Actor|GetComponentbyClass (.HitActor (Collision|BreakHitResult _outhit)) "/Game/Blueprints/Components/BPC_InteractableObject.BPC_InteractableObject_C"))))
                (if _result_2
                  (Actor|DestroyActor (.HitActor (Collision|BreakHitResult _outhit)))
                  (CallFunction|AddItemtoInventory _cell_2 (Variables|/Game/Blueprints/Components/BPC_InteractableObject.BPC_InteractableObject_C|GetItem (Actor|GetComponentbyClass (.HitActor (Collision|BreakHitResult _outhit)) "/Game/Blueprints/Components/BPC_InteractableObject.BPC_InteractableObject_C")) _index_2)
                  (else
                    (Default|Rotate (Variables|/Game/Blueprints/Components/BPC_InteractableObject.BPC_InteractableObject_C|GetItem (Actor|GetComponentbyClass (.HitActor (Collision|BreakHitResult _outhit)) "/Game/Blueprints/Components/BPC_InteractableObject.BPC_InteractableObject_C")))))))))))))

(fn GetAllItemsforCell
  (params (Cell :type BP%20Container%20Cell%20Object%20Reference))
  (for (_array_element _array_index) (Default|GetItems Cell)
    (if (not (.ReturnValue (Utilities|Map|Find (LocalVariables|GetLocalItems) _array_element)))
      (Utilities|Map|Add (LocalVariables|GetLocalItems) _array_element _array_index)
      (Development|PrintString "VALID")))
  (return (LocalVariables|GetLocalItems)))

(fn CanStoreIteminCellatLocation
  (params (Cell :type BP%20Container%20Cell%20Object%20Reference) (Item :type BP%20Container%20Item%20Object%20Reference) (X :type Integer) (Y :type Integer))
  (bind _dimension (Default|GetDimensions Item))
  (bind _dimensions (Default|GetDimensions Cell))
  (bind _dimension_2 (Default|GetDimensions Item))
  (if (and (>= (.x _dimensions) (+ (.x _dimension) X)) (>= (.y _dimensions) (+ (.y _dimension) Y)))
    (LocalVariables|SetLocalValid true)
    (bind _index (Utilities|FlowControl|ForLoopwithBreak X (+ (- (.x _dimension_2) 1) X) :!label _label)
      (:LoopBody
        (for _index_2 (range Y (+ (- (.y _dimension_2) 1) Y))
          (if (Utilities|Array|IsValidIndex (Default|GetItems Cell) (+ (* (.x (Default|GetDimensions Cell)) _index_2) _index))
            (if (Utilities|IsValid (Utilities|Array|Get(acopy) (Default|GetItems Cell) (+ (* (.x (Default|GetDimensions Cell)) _index_2) _index)))
              (LocalVariables|SetLocalValid false)
              (goto _label Break))
            (else
              (return 0 0 false)))))
      (:Completed
        (if (LocalVariables|GetLocalValid)
          (return X Y true)
          (else
            (return 0 0 false)))))
    (else
      (return 0 0 false))))

(fn RemoveItem
  (params (Item :type BP%20Container%20Item%20Object%20Reference) (FromCell :type BP%20Container%20Cell%20Object%20Reference))
  (for (_array_element _array_index) (Default|GetItems FromCell)
    (if (== _array_element Item)
      (Default|RemoveItematIndex FromCell _array_index)
      (Default|CallOnInventoryUpdated))))

(fn AddItemtoCellatLocation
  (params (Cell :type BP%20Container%20Cell%20Object%20Reference) (Item :type BP%20Container%20Item%20Object%20Reference) (Location :type Int%20Point%20Structure))
  (bind (_x _y) (Utilities|Struct|BreakIntPoint Location))
  (bind _dimension (Default|GetDimensions Item))
  (bind (_x_2 _y_2) (Utilities|Struct|BreakIntPoint _dimension))
  (for _index (range _x (+ _x (- _x_2 1)))
    (for _index_2 (range _y (+ _y (- _y_2 1)))
      (Default|SetItematIndex Cell Item (+ (* (.X (Utilities|Struct|BreakIntPoint (Default|GetDimensions Cell))) _index_2) _index))
      (Default|CallOnInventoryUpdated))))

(fn DropItemfromInventory
  (params (Item :type BP%20Container%20Item%20Object%20Reference))
  (Game|SpawnActorfromClass (Default|GetActortoSpawn Item) (Math|Transform|MakeTransform (Transformation|GetActorLocation (Variables|Default|GetHeroRef)) "0, 0, 0" "1.000000,1.000000,1.000000") "Undefined" "MultiplyWithRoot" 0 0)
  (bind (_cell _container _index _result) (CallFunction|FindItem Item))
  (if _result
    (CallFunction|RemoveItem Item _cell)))

(fn FindItem
  (params (Item :type BP%20Container%20Item%20Object%20Reference))
  (bind _items (CallFunction|GetAllContainerItems))
  (for _array_element _items
    (for _array_element_2 (Default|GetRows _array_element)
      (for (_array_element_3 _array_index) (Utilities|Struct|BreakS_ContainerRow _array_element_2)
        (if (Utilities|Array|ContainsItem (Default|GetItems _array_element_3) Item)
          (return _array_element_3 _array_element _array_index true)))))
  (return 0 0 0 false))

(fn HandleContainerItemAction
  (params (Action :type Enum_ContainerItemActions%20Enum :default "NewEnumerator0") (Item :type BP%20Container%20Item%20Object%20Reference) (FromCell :type BP%20Container%20Cell%20Object%20Reference))
  (switch Utilities|FlowControl|Switch|SwitchonEnum_ContainerItemActions Action
    (:NewEnumerator2
      (CallFunction|DropItemfromInventory Item)
      (CallFunction|RemoveItem Item FromCell))))

(fn RemoveEquippedItem
  (params (Item :type BP%20Container%20Item%20Object%20Reference))
  (Utilities|FlowControl|Sequence
    (:then_0
      (switch Utilities|FlowControl|Switch|SwitchonEnum_ContainerSlotType (Default|GetContainerSlotType Item)
        (:NewEnumerator0
          (Variables|Slots|SetSecretPocketSlot 0))))
    (:then_1
      (Default|CallOnInventoryUpdated))))

(fn GetAllSlots
  (return (Utilities|Array|MakeArray (Variables|Slots|GetSecretPocketSlot))))

(fn GetItemsfromItem
  (params (Item :type BP%20Container%20Item%20Object%20Reference))
  (for _array_element (Default|GetRows Item)
    (for _array_element_2 (Utilities|Struct|BreakS_ContainerRow _array_element)
      (bind _items (CallFunction|GetAllItemsforCell _array_element_2))
      (bind _keys (Utilities|Map|Keys _items))
      (for _array_element_3 _keys
        (Utilities|Array|Add (LocalVariables|GetLocalItems) _array_element_3))))
  (if (Utilities|Array|IsEmpty (LocalVariables|GetLocalItems))
    (return 0)
    (else
      (for _array_element_4 (LocalVariables|GetLocalItems)
        (bind _items_2 (CallFunction|GetItemsfromItem _array_element_4))
        (for _array_element_5 _items_2
          (Utilities|Array|Add (LocalVariables|GetLocalItems) _array_element_5)))
      (return (LocalVariables|GetLocalItems)))))

(fn EquipItematSlot
  (params (Item :type BP%20Container%20Item%20Object%20Reference))
  (Utilities|FlowControl|Sequence
    (:then_0
      (switch Utilities|FlowControl|Switch|SwitchonEnum_ContainerSlotType (Default|GetContainerSlotType Item)
        (:NewEnumerator0
          (Variables|Slots|SetSecretPocketSlot Item))))
    (:then_1
      (Default|CallOnInventoryUpdated))))