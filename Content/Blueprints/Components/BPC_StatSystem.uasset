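; Hero stat component that lets the player spend available points on a nested tree of Body, Mind, Soul and Luck stats.
; On BeginPlay it builds the stat tree, adds a screen-space WBP_StatUI to the owning BP_Hero_Base and binds its buttons.
; Clicks upgrade stats, deduct points and broadcast updates, with main-stat thresholds unlocking sub stats.
; Tertiary stats are only defined, UpdateStatData is deprecated, and debug keys add points or switch widget visibility.
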(event Custom|OnMainStatButtonClicked
  (params (StatType :type Enum_MainStatType%20Enum :default "NewEnumerator4") (AddAmount :type Integer))
  ;[0.15 0.15 0.15 0.5] Bind To Main Stat Button Clicked Event
  (if (> (Variables|Default|GetAvailablePoints) 0)
    (bind _upgradedstatidx (CallFunction|UpgradeMainStat StatType AddAmount))
    (bind _newavailablepoints (CallFunction|SubtractPoints AddAmount))
    (Default|CallAvailablePointsUpdated _newavailablepoints)
    (Default|CallMainStatUpdated (.Points (Utilities|Struct|BreakS_MainStat (Utilities|Array|Get(acopy) (Variables|Default|GetMainStats) _upgradedstatidx))) (.StatType (Utilities|Struct|BreakS_MainStat (Utilities|Array|Get(acopy) (Variables|Default|GetMainStats) _upgradedstatidx))))
    (else
      (Development|PrintString "No more points" true true "(R=1.000000,G=0.088960,B=0.029236,A=1.000000)" 5.0))))

(event Custom|OnSubStatButtonClicked
  (params (MainStatType :type Enum_MainStatType%20Enum :default "NewEnumerator4") (SubStatType :type Enum_SubStatType%20Enum :default "NewEnumerator0") (Amount :type Integer))
  ;[0.15 0.15 0.15 0.5] Bind To Sub Stat Button Clicked Event
  (if (> (Variables|Default|GetAvailablePoints) 0)
    (bind (_mainstatidx _upgradedstatidx) (CallFunction|UpgradeSubStat MainStatType SubStatType Amount))
    (bind _newavailablepoints (CallFunction|SubtractPoints Amount))
    (Default|CallAvailablePointsUpdated _newavailablepoints)
    (Default|CallSubStatUpdated (.Points (Utilities|Struct|BreakS_SubStat (Utilities|Array|Get(acopy) (Utilities|Struct|BreakS_MainStat (Utilities|Array|Get(acopy) (Variables|Default|GetMainStats) _mainstatidx)) _upgradedstatidx))) (.SubStatType (Utilities|Struct|BreakS_SubStat (Utilities|Array|Get(acopy) (Utilities|Struct|BreakS_MainStat (Utilities|Array|Get(acopy) (Variables|Default|GetMainStats) _mainstatidx)) _upgradedstatidx))))
    (else
      (Development|PrintString "No more points" true true "(R=1.000000,G=0.088960,B=0.029236,A=1.000000)" 5.0))))

(event EventBeginPlay
  (Utilities|FlowControl|Sequence
    (:then_0
      ;[0.15 0.15 0.15 0.5] Currently Init Main and Sub Stats
      (CallFunction|InitStats))
    (:then_1
      ;[0.15 0.15 0.15 0.5] Add Stat Wedgit to Player and Render It
      (bind _asbp_hero_base (Utilities|Casting|CastToBP_Hero_Base (Components|GetOwner)))
      (bind _output_get (Variables|Default|SetHeroRef _asbp_hero_base))
      (bind _returnvalue (Game|AddComponentbyClass _output_get "/Script/UMG.WidgetComponent" false))
      (Class|WidgetComponent|SetWidgetSpace _returnvalue "Screen")
      (Class|WidgetComponent|SetDrawSize _returnvalue "(X=1980.000000,Y=1080.000000)")
      (Variables|Default|SetStatWidgetComponent _returnvalue)
      (CallFunction|RenderStatWidget))
    (:then_2
      ;[0.15 0.15 0.15 0.5] Bind To Main Stat Button Clicked Event
      (bind _aswbp_stat_ui (Utilities|Casting|CastToWBP_StatUI (UserInterface|GetWidget (Variables|Default|GetStatWidgetComponent))))
      (EventDispatchers|BindEventtoMainStatButtonClicked _aswbp_stat_ui (delegate Custom|OnMainStatButtonClicked)))
    (:then_3
      ;[0.15 0.15 0.15 0.5] Bind To Sub Stat Button Clicked Event
      (bind _aswbp_stat_ui_2 (Utilities|Casting|CastToWBP_StatUI (UserInterface|GetWidget (Variables|Default|GetStatWidgetComponent))))
      (EventDispatchers|BindEventtoSubStatButtonClicked _aswbp_stat_ui_2 (delegate Custom|OnSubStatButtonClicked)))))

(event Input|KeyboardEvents|U
  (params (Key :type Key%20Structure :default "None"))
  ;[0.15 0.15 0.15 0.5] Testing
  (:Pressed
    (CallFunction|AddPoints 1)
    (Default|CallAvailablePointsUpdated (Variables|Default|GetAvailablePoints))))

(event Input|KeyboardEvents|I
  (params (Key :type Key%20Structure :default "None"))
  (:Pressed
    (if (Class|WidgetComponent|IsWidgetVisible (Variables|Default|GetStatWidgetComponent))
      (Class|WidgetComponent|SetWindowVisibility (Variables|Default|GetStatWidgetComponent) "SelfHitTestInvisible")
      (else
        (Class|WidgetComponent|SetWindowVisibility (Variables|Default|GetStatWidgetComponent) "Visible")))))

(fn UpdateStatData
  (params (StatType :type Enum_MainStatType%20Enum :default "NewEnumerator4") (Amount :type Integer))
  ;[0.15 0.15 0.15 0.5] Deprcated
  (switch Utilities|FlowControl|Switch|SwitchonEnum_MainStatType StatType
    (:NewEnumerator0
      (Utilities|Struct|SetmembersinS_StatData (Variables|Default|GetStatData) (+ (Utilities|Struct|BreakS_StatData (Variables|Default|GetStatData)) Amount))
      (if (< (Utilities|Struct|BreakS_StatData (Variables|Default|GetStatData)) 0)
        (Utilities|Struct|SetmembersinS_StatData (Variables|Default|GetStatData))
        (else
          (Development|PrintString (Utilities|String|Append "Update Body stat: " (Utilities|String|ToString(Integer) (Utilities|Struct|BreakS_StatData (Variables|Default|GetStatData))))))))
    (:NewEnumerator1
      (Utilities|Struct|SetmembersinS_StatData (Variables|Default|GetStatData) (+ (Utilities|Struct|BreakS_StatData (Variables|Default|GetStatData)) Amount))
      (if (< (Utilities|Struct|BreakS_StatData (Variables|Default|GetStatData)) 0)
        (Utilities|Struct|SetmembersinS_StatData (Variables|Default|GetStatData))
        (else
          (Development|PrintString (Utilities|String|Append "Update Mind stat: " (Utilities|String|ToString(Integer) (Utilities|Struct|BreakS_StatData (Variables|Default|GetStatData))))))))
    (:NewEnumerator2
      (Utilities|Struct|SetmembersinS_StatData (Variables|Default|GetStatData) (+ (Utilities|Struct|BreakS_StatData (Variables|Default|GetStatData)) Amount))
      (if (< (Utilities|Struct|BreakS_StatData (Variables|Default|GetStatData)) 0)
        (Utilities|Struct|SetmembersinS_StatData (Variables|Default|GetStatData))
        (else
          (Development|PrintString (Utilities|String|Append "Update Soul stat: " (Utilities|String|ToString(Integer) (Utilities|Struct|BreakS_StatData (Variables|Default|GetStatData))))))))
    (:NewEnumerator3
      (Utilities|Struct|SetmembersinS_StatData (Variables|Default|GetStatData) (+ (Utilities|Struct|BreakS_StatData (Variables|Default|GetStatData)) Amount))
      (if (< (Utilities|Struct|BreakS_StatData (Variables|Default|GetStatData)) 0)
        (Utilities|Struct|SetmembersinS_StatData (Variables|Default|GetStatData))
        (else
          (Development|PrintString (Utilities|String|Append "Update Luck stat: " (Utilities|String|ToString(Integer) (Utilities|Struct|BreakS_StatData (Variables|Default|GetStatData))))))))))

(fn RenderStatWidget
  (bind _returnvalue (UserInterface|CreateWidget "/Game/Blueprints/Widgets/WBP_StatUI.WBP_StatUI_C"))
  (UserInterface|SetWidget (Variables|Default|GetStatWidgetComponent) _returnvalue))

(fn AddPoints
  (params (Amount :type Integer))
  (Variables|Default|SetAvailablePoints (+ (Variables|Default|GetAvailablePoints) Amount))
  (Development|PrintString (Utilities|String|Append "Add " (Utilities|String|ToString(Integer) Amount) " points to StatSystem"))
  (return (Variables|Default|GetAvailablePoints)))

(fn UpgradeMainStat
  (params (StatType :type Enum_MainStatType%20Enum :default "NewEnumerator4") (Amount :type Integer))
  ;[0.15 0.15 0.15 0.5] Get the Main Stat and upgrade it by Amount
  (for (_ _array_index) (Variables|Default|GetMainStats)
    (LocalVariables|SetTargetIdx _array_index)
    (if (Utilities|Enum|Equal(Enum) (.StatType (Utilities|Struct|BreakS_MainStat (Utilities|Array|Get(acopy) (Variables|Default|GetMainStats) (LocalVariables|GetTargetIdx)))) StatType)
      (Utilities|Struct|SetmembersinS_MainStat (Utilities|Array|Get(acopy) (Variables|Default|GetMainStats) (LocalVariables|GetTargetIdx)) (+ Amount (.Points (Utilities|Struct|BreakS_MainStat (Utilities|Array|Get(acopy) (Variables|Default|GetMainStats) (LocalVariables|GetTargetIdx))))))
      ;[0.15 0.15 0.15 0.5] Check if the MainStat's substats are unlocked
      (if (and (>= (.Points (Utilities|Struct|BreakS_MainStat (Utilities|Array|Get(acopy) (Variables|Default|GetMainStats) (LocalVariables|GetTargetIdx)))) (.PointsToUnlockSub (Utilities|Struct|BreakS_MainStat (Utilities|Array|Get(acopy) (Variables|Default|GetMainStats) (LocalVariables|GetTargetIdx))))) (not (.IsSubStatsUnlocked (Utilities|Struct|BreakS_MainStat (Utilities|Array|Get(acopy) (Variables|Default|GetMainStats) (LocalVariables|GetTargetIdx))))))
        (bind _structout (Utilities|Struct|SetmembersinS_MainStat (Utilities|Array|Get(acopy) (Variables|Default|GetMainStats) (LocalVariables|GetTargetIdx)) true))
        (Default|CallSubStatsUnlocked (.StatType (Utilities|Struct|BreakS_MainStat _structout)))
        ;[0.15 0.15 0.15 0.5] Unlock Sub Stats if the Main Stat reach the required unlock points
        (for (_ _array_index_2) (.SubStats (Utilities|Struct|BreakS_MainStat (Utilities|Array|Get(acopy) (Variables|Default|GetMainStats) (LocalVariables|GetTargetIdx))))
          (Utilities|Struct|SetmembersinS_SubStat (Utilities|Array|Get(acopy) (.SubStats (Utilities|Struct|BreakS_MainStat (Utilities|Array|Get(acopy) (Variables|Default|GetMainStats) (LocalVariables|GetTargetIdx)))) _array_index_2) true))
        (Development|PrintString (Utilities|String|Append "Unlock  " (Utilities|String|EnumtoString (.StatType (Utilities|Struct|BreakS_MainStat (Utilities|Array|Get(acopy) (Variables|Default|GetMainStats) (LocalVariables|GetTargetIdx))))) "'s substats") true true "(R=1.000000,G=0.000000,B=0.068093,A=1.000000)" 5.0)
        (return (LocalVariables|GetTargetIdx))
        (else
          (return (LocalVariables|GetTargetIdx))))))
  (Development|PrintString "Didn't find a Stat to upgrade"))

(fn InitStats
  (Variables|Default|SetMainStats (Utilities|Array|MakeArray (Utilities|Struct|MakeS_MainStat "Body" 0 "NewEnumerator0" (Variables|UnlockStatPointsBody|GetUnlockBodyPoints) false (Utilities|Array|MakeArray (Utilities|Struct|MakeS_SubStat "Power" "NewEnumerator0" (Variables|UnlockStatPointsBody|GetUnlockPowerPoints) (Utilities|Array|MakeArray (Utilities|Struct|MakeS_TertiaryStat "Piercing" "NewEnumerator0") (Utilities|Struct|MakeS_TertiaryStat "Bludgeoning" "NewEnumerator1") (Utilities|Struct|MakeS_TertiaryStat "Slashing" "NewEnumerator2") (Utilities|Struct|MakeS_TertiaryStat "StunChance" "NewEnumerator3") (Utilities|Struct|MakeS_TertiaryStat "BleedChance" "NewEnumerator4") (Utilities|Struct|MakeS_TertiaryStat "Initmidation" "NewEnumerator5"))) (Utilities|Struct|MakeS_SubStat "Speed" "NewEnumerator1") (Utilities|Struct|MakeS_SubStat "Vigor" 0 "NewEnumerator2") (Utilities|Struct|MakeS_SubStat "Endurance" 0 "NewEnumerator3"))) (Utilities|Struct|MakeS_MainStat "Mind" 0 "NewEnumerator1" (Variables|UnlockStatPointsMind|GetUnlockMindPoints) false (Utilities|Array|MakeArray (Utilities|Struct|MakeS_SubStat "Intelligence" 0 "NewEnumerator9") (Utilities|Struct|MakeS_SubStat "Wisdom" 0 "NewEnumerator10") (Utilities|Struct|MakeS_SubStat "Charisma" 0 "NewEnumerator11"))) (Utilities|Struct|MakeS_MainStat "Soul" 0 "NewEnumerator2" (Variables|UnlockStatPointsSoul|GetUnlockSoulPoints) false (Utilities|Array|MakeArray (Utilities|Struct|MakeS_SubStat "Magic" 0 "NewEnumerator12") (Utilities|Struct|MakeS_SubStat "Mana" 0 "NewEnumerator13") (Utilities|Struct|MakeS_SubStat "Faith" 0 "NewEnumerator14") (Utilities|Struct|MakeS_SubStat "Devotion" 0 "NewEnumerator15"))) (Utilities|Struct|MakeS_MainStat "Luck" 0 "NewEnumerator3" (Variables|UnlockStatPointsLuck|GetUnlockLuckPoints) false (Utilities|Array|MakeArray (Utilities|Struct|MakeS_SubStat "DropChance" 0 "NewEnumerator16") (Utilities|Struct|MakeS_SubStat "PhysicalCritChance" 0 "NewEnumerator17") (Utilities|Struct|MakeS_SubStat "MagicCritChance" 0 "NewEnumerator18") (Utilities|Struct|MakeS_SubStat "DropCHance" 0 "NewEnumerator16")))))
  (Development|PrintString "Stats Setup"))

(fn UpgradeSubStat
  (params (MainStatType :type Enum_MainStatType%20Enum :default "NewEnumerator4") (SubStatType :type Enum_SubStatType%20Enum :default "NewEnumerator0") (Amount :type Integer))
  ;[0.15 0.15 0.15 0.5] Get the Main Stat
  (for (_array_element _array_index) (Variables|Default|GetMainStats)
    (LocalVariables|SetTargetMainStatIdx _array_index)
    (if (Utilities|Enum|Equal(Enum) (Utilities|Struct|BreakS_MainStat _array_element) MainStatType)
      ;[0.15 0.15 0.15 0.5] Get the SubStat
      (bind (_substatidx _succeed) (CallFunction|GetSubStatIdx _array_element SubStatType))
      (LocalVariables|SetTargetSubStatIdx _substatidx)
      (if _succeed
        ;[0.15 0.15 0.15 0.5] If the SubStat is unlocked
        (if (.IsUnlocked (Utilities|Struct|BreakS_SubStat (Utilities|Array|Get(acopy) (Utilities|Struct|BreakS_MainStat (Utilities|Array|Get(acopy) (Variables|Default|GetMainStats) (LocalVariables|GetTargetMainStatIdx))) (LocalVariables|GetTargetSubStatIdx))))
          ;[0.15 0.15 0.15 0.5] Upgrade the SubStat by Amount
          (Utilities|Struct|SetmembersinS_SubStat (Utilities|Array|Get(acopy) (Utilities|Struct|BreakS_MainStat (Utilities|Array|Get(acopy) (Variables|Default|GetMainStats) (LocalVariables|GetTargetMainStatIdx))) (LocalVariables|GetTargetSubStatIdx)) (+ (Utilities|Struct|BreakS_SubStat (Utilities|Array|Get(acopy) (Utilities|Struct|BreakS_MainStat (Utilities|Array|Get(acopy) (Variables|Default|GetMainStats) (LocalVariables|GetTargetMainStatIdx))) (LocalVariables|GetTargetSubStatIdx))) Amount))
          (return (LocalVariables|GetTargetMainStatIdx) (LocalVariables|GetTargetSubStatIdx))
          (else
            (Development|PrintString (Utilities|String|Append (Utilities|String|EnumtoString (.SubStatType (Utilities|Struct|BreakS_SubStat (Utilities|Array|Get(acopy) (Utilities|Struct|BreakS_MainStat (Utilities|Array|Get(acopy) (Variables|Default|GetMainStats) (LocalVariables|GetTargetMainStatIdx))) (LocalVariables|GetTargetSubStatIdx))))) " is not unlocked"))))))))

(fn SubtractPoints
  (params (Amount :type Integer))
  (Variables|Default|SetAvailablePoints (- (Variables|Default|GetAvailablePoints) Amount))
  (Development|PrintString (Utilities|String|Append "Subtract  " (Utilities|String|ToString(Integer) Amount) " points from StatSystem"))
  (return (Variables|Default|GetAvailablePoints)))