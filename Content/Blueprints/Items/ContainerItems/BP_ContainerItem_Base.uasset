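; BP_ContainerItem_Base is, judging by its name, a base actor for container items, and it holds an Item reference.
; Its SetItem event stores the given Item on the actor and copies it to the BPCInteractableObject component, so both hold the same value.
; It adds no other logic: BeginPlay, overlap and Tick are disabled stubs, and the construction script only calls its parent.
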(event EventBeginPlay
  (|CallParentFunction) ; This node is disabled and will not be called.\nDrag off pins to build functionality.
)

(event Collision|EventActorBeginOverlap
  (params (OtherActor :type Actor%20Object%20Reference))
  (|CallParentFunction OtherActor) ; This node is disabled and will not be called.\nDrag off pins to build functionality.
)

(event EventTick
  (params (DeltaSeconds :type Float%20%28single-precision%29))
  (|CallParentFunction DeltaSeconds) ; This node is disabled and will not be called.\nDrag off pins to build functionality.
)

(event EventSetItem
  (params (Item :type BP%20Container%20Item%20Object%20Reference))
  (bind _output_get (Variables|Default|SetItem Item))
  (Variables|/Game/Blueprints/Components/BPC_InteractableObject.BPC_InteractableObject_C|SetItem (Variables|Default|GetBPC_InteractableObject) _output_get))

(fn ConstructionScript
  (|CallParentFunction))